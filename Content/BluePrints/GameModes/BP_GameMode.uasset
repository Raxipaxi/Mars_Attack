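; Game mode that runs endless waves of aliens with escalating difficulty.
; Each wave multiplies the difficulty to set the spawn count, then a looping timer spawns BP_Alien at random TargetPoints until that count runs out.
; Spawned aliens are tracked in an array, and registered deaths remove them.
; Once none remain alive or left to spawn, the next wave starts after a short delay.
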(event Custom|Spawn%20Wave
  (CallFunction|SpawnAlien))

(event Custom|End%20Wave
  (Utilities|FlowControl|Delay 2.0)
  (CallFunction|StartNewWave))

(event EventBeginPlay
  (Utilities|FlowControl|Delay 2.0)
  (CallFunction|StartNewWave))

(event EventTick
  (params (DeltaSeconds :type Float%20%28single-precision%29)))

(fn ConstructionScript)

(fn StartNewWave
  (Math|Integer|IncrementInt (Variables|Default|GetCurrent%20Wave)
    (:%20%20
      (CallFunction|AddDifficulty)
      (Utilities|Time|SetTimerbyFunctionName 0 "Spawn Wave" 1.0 true))))

(fn SpawnAlien
  (bind _output (CallFunction|GetRandomSpawnponint))
  (Utilities|IsValid _output
    (:Is%20Valid
      (bind _returnvalue (Game|SpawnActorfromClass "/Game/BluePrints/AI/BP_Alien.BP_Alien_C" (Transformation|GetActorTransform _output) "Undefined" 0 0))
      (Utilities|IsValid _returnvalue
        (:Is%20Valid
          (Utilities|Array|Add (Variables|Default|GetAlienArray) _returnvalue)
          (bind _result (Math|Integer|DecrementInt (Variables|Default|GetAliens%20Spawn%20Remaining))
            (:%20%20
              (if (== _result 0)
                (Utilities|Time|ClearTimerbyFunctionName 0 "Spawn Wave")))))))))

(fn GetRandomSpawnponint
  (bind _outactors (Actor|GetAllActorsOfClass "/Script/Engine.TargetPoint"))
  (return (Utilities|Array|Get(acopy) _outactors (Math|Random|RandomIntegerinRange 0 (Utilities|Array|LastIndex _outactors)))))

(fn RegisterAlienDeath
  (params (Alien :type BP%20Alien%20Object%20Reference%20%28by%20ref%29))
  (Utilities|Array|RemoveItem (Variables|Default|GetAlienArray) Alien)
  (if (CallFunction|IsWaveComplete)
    (CallFunction|EndWave)))

(fn IsWaveComplete
  (return (and (== (Utilities|Array|Length (Variables|Default|GetAlienArray)) 0) (== (Variables|Default|GetAliens%20Spawn%20Remaining) 0))))

(fn AddDifficulty
  (bind _output_get (Variables|Default|SetDifficulty (Math|Float|Round (* (Variables|Default|GetDifficulty) (Variables|Default|GetDifficulty%20Multiplier)))))
  (Variables|Default|SetAliens%20Spawn%20Remaining _output_get)
  (return))