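; Player marine pawn for a twin-stick shooter, with world-axis movement, health, death, a kill counter and a HUD.
; Each tick it sets control rotation from thumbstick angle or smoothed mouse velocity, both deadzoned, choosing by whether the pressed key is a gamepad key.
; Firing runs a looping timer of muzzle line traces along that rotation, applying damage and impact effects.
; Damage reaching zero health sets Dead, stopping fire and blocking movement and aim.
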(event EventBeginPlay
  ;[0.01757 0 1] HUD Creation
  (bind _returnvalue (UserInterface|CreateWidget "/Game/UI/W_PlayerHUD.W_PlayerHUD_C" 0 self))
  (UserInterface|Viewport|AddtoViewport _returnvalue 0))

(event EventTick
  (params (DeltaSeconds :type Float%20%28single-precision%29))
  ;[0.1706 1 0.8398] Aim
  (Weapon|UpdatePlayerAim (Class|KismetInputLibrary|KeyIsGamepadKey (stale Input|KeyboardEvents|AnyKey Key))))

(event Game|Damage|EventAnyDamage
  (params (Damage :type Float%20%28single-precision%29) (DamageType :type Damage%20Type%20Object%20Reference) (InstigatedBy :type Controller%20Object%20Reference) (DamageCauser :type Actor%20Object%20Reference))
  ;[1 0 0] Receive Damage
  (if (Health|IsAlive)
    (bind _health (Health|DecreaseHealth Damage))
    (if (== _health 0.0)
      (Variables|Default|SetDead true)
      (Weapon|StopFiringWeapon))))

(event Input|ActionEvents|InputActionFireWeapon
  (params (Key :type Key%20Structure :default "None"))
  ;[1 0.06197 0.05203] Shoot
  (:Pressed
    (Weapon|StartFiringWeapon))
  (:Released
    (Weapon|StopFiringWeapon)))

(event Input|AxisEvents|InputAxisMoveForward
  (params (AxisValue :type Float%20%28single-precision%29))
  ;[0.1706 1 0.8398] Movement
  (if (Health|IsAlive)
    (Pawn|Input|AddMovementInput "1.000000, 0, 0" AxisValue false)))

(event Input|AxisEvents|InputAxisMoveRight
  (params (AxisValue :type Float%20%28single-precision%29))
  ;[0.1706 1 0.8398] Movement
  (if (Health|IsAlive)
    (Pawn|Input|AddMovementInput "0,1.000000, 0" AxisValue false)))

(event Input|KeyboardEvents|AnyKey
  (params (Key :type Key%20Structure :default "None"))
  ;[0.1706 1 0.8398] Aim
  (:Pressed
    (Weapon|UpdatePlayerAim (Class|KismetInputLibrary|KeyIsGamepadKey Key))))

(fn ConstructionScript)

(fn UpdatePlayerAim
  (params (IsGamepad :type Boolean))
  (if (Health|IsAlive)
    (if IsGamepad
      (ThumbstickInput|UpdateThumbstickAim)
      (else
        (MouseInput|UpdateMouseAim)))))

(fn IsThimbstickAboveDeathzone
  (return (>= (Math|Vector2D|Vector2DLength (Math|Vector2D|MakeVector2D (Input|AxisValues|GetThumbstickAimUp) (Input|AxisValues|GetThumbstickAimRight))) (Variables|ThumbstickInput|GetThumbStickDeadZone))))

(fn SetMarineAimRotation
  (return (Math|Rotator|MakeRotator 0.0 0.0 (Class|KismetMathLibrary|DegAtan2 (Input|AxisValues|GetThumbstickAimRight) (Input|AxisValues|GetThumbstickAimUp)))))

(fn GetMouseVelocity
  (bind _returnvalue (Game|GetPlayerController 0))
  (bind (_deltax _deltay) (Class|PlayerController|GetInputMouseDelta _returnvalue))
  (return (/ (Math|Vector2D|MakeVector2D _deltax _deltay) (Utilities|Time|GetWorldDeltaSeconds))))

(fn MouseDeathZone
  (return (> (Math|Vector2D|Vector2DLength (MouseInput|GetMouseVelocity)) 2e+01)))

(fn UpdateMouseAim
  (if (MouseInput|MouseDeathZone)
    (Pawn|SetControlRotation (Game|GetPlayerController 0) (MouseInput|GetMouseAimDir))))

(fn GetMouseAimDir
  (bind _returnvalue (MouseInput|GetMouseVelocity))
  (return (Math|Interpolation|RInterpTo (Pawn|GetControlRotation (Game|GetPlayerController 0) :!class /Script/Engine.Controller) (Math|Rotator|MakeRotator 0.0 0.0 (Class|KismetMathLibrary|DegAtan2 (.x _returnvalue) (.y _returnvalue))) (Utilities|Time|GetWorldDeltaSeconds) (Variables|MouseInput|GetMouseSmoothing))))

(fn UpdateThumbstickAim
  (if (ThumbstickInput|IsThimbstickAboveDeathzone)
    (Pawn|SetControlRotation (Game|GetPlayerController 0) (ThumbstickInput|SetMarineAimRotation))))

(fn StartFiringWeapon
  (if (Health|IsAlive)
    (Components|Activation|Activate (Variables|Default|GetP_AssaultRifle_MF) false)
    (bind _returnvalue (Audio|SpawnSound2D "/Game/Sounds/Weapon_AssaultRifle/Stereo/RifleFireLoop_Cue.RifleFireLoop_Cue" 1.0 1.0 0.0 0))
    (Variables|Default|SetWeapon%20Fire%20Sound _returnvalue)
    (Weapon|WeaponTrace)
    (Utilities|Time|SetTimerbyFunctionName 0 "Weapon Trace" (Variables|Default|GetWeapon%20Fire%20Rate) true)))

(fn StopFiringWeapon
  (bind _weapon_fire_sound (Variables|Default|GetWeapon%20Fire%20Sound))
  (Components|Activation|Deactivate (Variables|Default|GetP_AssaultRifle_MF))
  (Utilities|IsValid _weapon_fire_sound
    (:Is%20Valid
      (Audio|Components|Audio|Stop _weapon_fire_sound)
      (Utilities|Time|ClearTimerbyFunctionName 0 "Weapon Trace")
      (if (Health|IsAlive)
        (Audio|SpawnSound2D "/Game/Sounds/Weapon_AssaultRifle/Stereo/RifleFireEnd_Cue.RifleFireEnd_Cue" 1.0 1.0 0.0 0)))))

(fn DecreaseHealth
  (params (Damage%20Amount :type Float%20%28single-precision%29))
  (bind _output_get (Variables|MarineStats|SetHealth (Math|Float|Clamp(Float) (- (Variables|MarineStats|GetHealth) Damage%20Amount) 0.0 1e+02)))
  (return _output_get))

(fn IsAlive
  (return (not (Variables|Default|GetDead))))

(fn WeaponTrace
  (bind _outhit (Collision|LineTraceByChannel (Weapon|GetWeaponStartLocation) (Weapon|GetWeaponEndLocation) "TraceTypeQuery1" false 0 "None"))
  (if (.bBlockingHit (Collision|BreakHitResult _outhit))
    (Weapon|SpawnImpactHit (.Location (Collision|BreakHitResult _outhit)))
    (Game|Damage|ApplyDamage (.HitActor (Collision|BreakHitResult _outhit)) (Variables|Default|GetDamage%20per%20shot) 0 0)))

(fn GetWeaponStartLocation
  (return (Transformation|GetSocketLocation (Variables|Default|GetRifle) "MuzzleFlash")))

(fn GetWeaponEndLocation
  (return (+ (Weapon|GetWeaponStartLocation) (* (Math|Vector|GetForwardVector (Pawn|GetControlRotation :!class /Script/Engine.Pawn)) (Variables|Default|GetWeapon%20Range)))))

(fn IncreaseKillls
  (Math|Integer|IncrementInt (Variables|MarineStats|GetEnemyKills)))

(fn SpawnImpactHit
  (params (ImpactHit :type Vector))
  (Effects|SpawnEmitteratLocation "/Game/Effects/Weapons/Impacts/P_AssaultRifle_IH.P_AssaultRifle_IH" ImpactHit))

(fn AddHealth
  (params (Heal :type Float%20%28single-precision%29))
  (Variables|MarineStats|SetHealth (Math|Float|Clamp(Float) (+ Heal (Variables|MarineStats|GetHealth)) 0.0 1e+02)))

(fn IsHealthFull
  (return (== (Variables|MarineStats|GetHealth) 1e+02)))