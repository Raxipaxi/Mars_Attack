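; Enemy alien character that chases the first player and melees when in range.
; BeginPlay runs a repeating AI MoveTo loop, while Tick checks range and plays an attack montage with movement deactivated until completion.
; Damage lowers clamped health; at zero it disables movement and collision, credits BP_Marine's kill, notifies BP_GameMode and destroys itself after a delay.
; DamagePlayer applies hit damage but is not called within this Blueprint.
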(event EventBeginPlay
  ;[0 1 0.534] Setting Target
  (Variables|Default|SetTarget%20Player (Game|GetPlayerCharacter 0))
  ;[0.2393 0.9801 1] Chase
  (if (CallFunction|IsAlive) :!label _label
    (AI|AIMoveTo self "0, 0, 0" (Variables|Default|GetTarget%20Player) 5.0 false
      (:OnSuccess
        _)
      (:OnFail
        _))
    (Utilities|FlowControl|Delay 0.2)
    (goto _label)))

(event Game|Damage|EventAnyDamage
  (params (Damage :type Float%20%28single-precision%29) (DamageType :type Damage%20Type%20Object%20Reference) (InstigatedBy :type Controller%20Object%20Reference) (DamageCauser :type Actor%20Object%20Reference))
  (bind _output_get (CallFunction|ReceiveDamage Damage))
  (if (== _output_get 0.0)
    (CallFunction|KillAI)
    (Utilities|FlowControl|Delay 3.0)
    (Actor|DestroyActor)))

(event EventTick
  (params (DeltaSeconds :type Float%20%28single-precision%29))
  ;[1 0 0] Attack
  (if (CallFunction|CanAttack)
    (AI|DeactivateAIMovement)
    (Animation|Montage|PlayMontage (Variables|Character|GetMesh) "/Game/Characters/Enemy_Great_Spider/Animations/AlienAttck1.AlienAttck1"
      (:OnCompleted
        (AI|ActivateAIMovement)))))

(fn ConstructionScript)

(fn IsWithinAttackRange
  (return (< (Transformation|GetDistanceTo (Variables|Default|GetTarget%20Player)) (Variables|Default|GetAttackRange))))

(fn IsAttacking
  (return (Animation|Montage|MontageIsPlaying (Components|SkeletalMesh|GetAnimInstance (Variables|Character|GetMesh)) "/Game/Characters/Enemy_Great_Spider/Animations/AlienAttck1.AlienAttck1")))

(fn DeactivateAIMovement
  (bind _charactermovement (Variables|Character|GetCharacterMovement))
  (Components|Movement|StopMovementImmediately _charactermovement)
  (Components|Activation|Deactivate _charactermovement))

(fn ActivateAIMovement
  (Components|Activation|Activate (Variables|Character|GetCharacterMovement) false))

(fn DamagePlayer
  (if (CallFunction|IsAlive)
    (Game|Damage|ApplyDamage (Variables|Default|GetTarget%20Player) (Variables|Default|GetDamage%20per%20hit) 0 0)))

(fn ReceiveDamage
  (params (Damage :type Float%20%28single-precision%29))
  (if (CallFunction|IsAlive)
    (bind _output_get (Variables|Default|SetHealth (Math|Float|Clamp(Float) (- (Variables|Default|GetHealth) Damage) 0.0 1e+02)))
    (return _output_get)))

(fn KillAI
  (Variables|Default|SetDead true)
  (AI|DeactivateAIMovement)
  (Collision|SetActorEnableCollision false)
  (bind _asbp_marine (Utilities|Casting|CastToBP_Marine (Game|GetPlayerCharacter 0)))
  (Default|IncreaseKillls _asbp_marine)
  (bind _asbp_game_mode (Utilities|Casting|CastToBP_GameMode (Game|GetGameMode)))
  (Default|RegisterAlienDeath _asbp_game_mode self))

(fn IsAlive
  (return (not (Variables|Default|GetDead))))

(fn CanAttack
  (return (Math|Boolean|ANDBoolean (AI|IsWithinAttackRange) (not (AI|IsAttacking)) (CallFunction|IsAlive))))